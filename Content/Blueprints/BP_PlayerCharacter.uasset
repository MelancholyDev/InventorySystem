(event `Key|E`
  (params (Key :type "Key Structure"))
  (:`Pressed`
    (`/Game/Blueprints/Components/BP_InventoryComponent.AddItem` (`self.BP_InventoryComponent`))))

(event `Key|I`
  (params (Key :type "Key Structure"))
  (:`Pressed`
    (message `/Game/Blueprints/Interfaces/BPI_UI.ToggleInventory` (`PlayerController.GetHUD` (`GameplayStatics.GetPlayerController` 0)))))

(event `Key|RightMouseButton`
  (params (Key :type "Key Structure"))
  (:`Pressed`
    (`/Game/Blueprints/Components/BP_InventoryComponent.UseRightSlot` (`self.BP_InventoryComponent`))))

(event `Key|LeftMouseButton`
  (params (Key :type "Key Structure"))
  (:`Pressed`
    (`/Game/Blueprints/Components/BP_InventoryComponent.UseLeftSlot` (`self.BP_InventoryComponent`))))

(event `Key|One`
  (params (Key :type "Key Structure"))
  (:`Pressed`
    (`/Game/Blueprints/Components/BP_ResourceHealthComponent.ChangeHealth` (`self.BP_ResourceHealthComponent`) -10)))

(fn `UserConstructionScript`)