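; Interact component that keeps a list of quest-usable items and triggers their use.
; AddItem and DeleteItem maintain the QuestUsableItems array.
; UseItem takes the first entry if valid and calls its UseMessage, first removing it from the list when the item is flagged OneUse.
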(fn `AddItem`
  (params (Item :type "/Game/Blueprints/UsableItems/BP_UsableWithQuestItem Object Reference"))
  (`KismetArrayLibrary.Array_Add` (`self.QuestUsableItems`) Item))

(fn `DeleteItem`
  (params (Item :type "/Game/Blueprints/UsableItems/BP_UsableWithQuestItem Object Reference"))
  (`KismetArrayLibrary.Array_RemoveItem` (`self.QuestUsableItems`) Item))

(fn `UseItem`
  (locals (ItemToIse :type "/Game/Blueprints/UsableItems/BP_UsableWithQuestItem Object Reference"))
  (bind _output (`|GetArrayItem` (`self.QuestUsableItems`)))
  (`/Engine/EditorBlueprintResources/StandardMacros.IsValid` _output
    (:`Is Valid`
      (bind _output_get (set `local.ItemToIse` _output))
      (if (`/Game/Blueprints/UsableItems/BP_UsableWithQuestItem.OneUse` _output_get)
        (`KismetArrayLibrary.Array_RemoveItem` (`self.QuestUsableItems`) (`local.ItemToIse`))
        (message `/Game/Blueprints/Interfaces/BPI_UsableItem.Use` (`local.ItemToIse`))
        (else
          (message `/Game/Blueprints/Interfaces/BPI_UsableItem.Use` (`local.ItemToIse`)))))))