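; BP_SpawnZone scatters a set number of collectable items on surfaces inside a box volume.
; Spawn clears earlier results, then adds a child actor component per item and line-traces on Visibility from the box top at seeded random XY points.
; On a hit, the component moves to the impact location, becomes a BP_CollectableItem and is initialized with the zone's Item data.
; DestroyAll removes every tracked component.
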(fn `DestroyAll`
  (locals (Component :type "ChildActorComponent Object Reference"))
  (while (> (`KismetArrayLibrary.Array_Length` (`self.Actors`)) 0)
    (set `local.Component` (`|GetArrayItem` (`self.Actors`)))
    (`KismetArrayLibrary.Array_Remove` (`self.Actors`))
    (`ActorComponent.K2_DestroyComponent` (`local.Component`))))

(fn `Spawn`
  (locals (SpawnedActor :type "ChildActorComponent Object Reference"))
  (bind _spawnedactor (`local.SpawnedActor`))
  (bind (_returnvalue_x _returnvalue_y _returnvalue_z) (`KismetMathLibrary.BreakVector` (`SceneComponent.K2_GetComponentLocation` (`self.Box`))))
  (bind (_returnvalue_x_2 _returnvalue_y_2 _returnvalue_z_2) (`KismetMathLibrary.BreakVector` (`BoxComponent.GetScaledBoxExtent` (`self.Box`))))
  (bind _returnvalue (+ _returnvalue_z_2 _returnvalue_z))
  (bind _x (.x (`KismetMathLibrary.RandomPointInBoundingBoxFromStream` (`SceneComponent.K2_GetComponentLocation` (`self.Box`)) (`BoxComponent.GetScaledBoxExtent` (`self.Box`)) (`self.RandomSeed`))))
  (bind _y (.y (`KismetMathLibrary.RandomPointInBoundingBoxFromStream` (`SceneComponent.K2_GetComponentLocation` (`self.Box`)) (`BoxComponent.GetScaledBoxExtent` (`self.Box`)) (`self.RandomSeed`))))
  (`self.DestroyAll`)
  (for _ (range (`self.Num`))
    (bind _returnvalue_2 (`AddComponent|NODE_AddChildActorComponent-1`))
    (bind _output_get (set `local.SpawnedActor` _returnvalue_2))
    (`KismetArrayLibrary.Array_Add` (`self.Actors`) _output_get)
    (bind (_outhit _returnvalue_3) (`KismetSystemLibrary.LineTraceSingle` (`KismetMathLibrary.MakeVector` _x _y _returnvalue) (+ (`KismetMathLibrary.MakeVector` _x _y _returnvalue) (`KismetMathLibrary.MakeVector` 0.0 0.0 (* _returnvalue_z_2 -2.0))) "TraceTypeQuery1"))
    (if _returnvalue_3
      (`SceneComponent.K2_SetWorldLocation` (`local.SpawnedActor`) (`.Location` (`GameplayStatics.BreakHitResult` _outhit)) false false)
      (`ChildActorComponent.SetChildActorClass` _spawnedactor "/Game/Blueprints/Items/BP_CollectableItem.BP_CollectableItem_C")
      (bind _asbp_collectable_item (cast `/Game/Blueprints/Items/BP_CollectableItem` (`ChildActorComponent.ChildActor` _spawnedactor)))
      (set `/Game/Blueprints/Items/BP_CollectableItem.ItemData` (`self.Item`) _asbp_collectable_item)
      (`/Game/Blueprints/Items/BP_CollectableItem.CreateItem` _asbp_collectable_item))))

(fn `UserConstructionScript`)