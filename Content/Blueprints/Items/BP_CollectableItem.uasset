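; BP_CollectableItem is a world pickup that the player's inventory can collect.
; Its construction script reads the item's data table row and spawns a static or skeletal mesh component based on the row's AdditionalData asset class, applying scale and an optional override material for static meshes.
; Box overlaps by the player pawn register or unregister the item with BP_InventoryComponent as a pickup candidate.
; PickUp simply destroys the actor.
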(event `self.Box.OnComponentBeginOverlap`
  (params (OverlappedComponent :type "PrimitiveComponent Object Reference") (OtherActor :type "Actor Object Reference") (OtherComp :type "PrimitiveComponent Object Reference") (OtherBodyIndex :type Integer) (bFromSweep :type Boolean) (SweepResult :type "HitResult Structure (by ref)"))
  (bind _returnvalue (`self.GetComponentByClass` (`GameplayStatics.GetPlayerPawn` 0) "/Game/Blueprints/Components/BP_InventoryComponent.BP_InventoryComponent_C"))
  (if (== OtherActor (`GameplayStatics.GetPlayerPawn` 0))
    (`/Engine/EditorBlueprintResources/StandardMacros.IsValid` _returnvalue
      (:`Is Valid`
        (`/Game/Blueprints/Components/BP_InventoryComponent.AddPickupItem` _returnvalue self)))))

(event `self.Box.OnComponentEndOverlap`
  (params (OverlappedComponent :type "PrimitiveComponent Object Reference") (OtherActor :type "Actor Object Reference") (OtherComp :type "PrimitiveComponent Object Reference") (OtherBodyIndex :type Integer))
  (bind _returnvalue (`self.GetComponentByClass` (`GameplayStatics.GetPlayerPawn` 0) "/Game/Blueprints/Components/BP_InventoryComponent.BP_InventoryComponent_C"))
  (if (== OtherActor (`GameplayStatics.GetPlayerPawn` 0))
    (`/Engine/EditorBlueprintResources/StandardMacros.IsValid` _returnvalue
      (:`Is Valid`
        (`/Game/Blueprints/Components/BP_InventoryComponent.DeletePickupItem` _returnvalue self)))))

(fn `AddSkeletalMesh`
  (bind _aspda_skeletal_mesh_item (cast `/Game/Assets/DataAssets/PrimaryDataAssets/PDA_SkeletalMeshItem` (`self.AdditionalData`)))
  (bind _returnvalue (`AddComponent|NODE_AddSkeletalMeshComponent-1`))
  (`SkinnedMeshComponent.SetSkinnedAssetAndUpdate` _returnvalue (`/Game/Assets/DataAssets/PrimaryDataAssets/PDA_SkeletalMeshItem.SkeletalMesh` _aspda_skeletal_mesh_item) true))

(fn `AddStaticMesh`
  (locals (StaticMeshData :type "/Game/Assets/DataAssets/PrimaryDataAssets/PDA_StaticMeshItem Object Reference"))
  (bind _overridematerial (`/Game/Assets/DataAssets/PrimaryDataAssets/PDA_StaticMeshItem.OverrideMaterial` (`local.StaticMeshData`)))
  (bind _aspda_static_mesh_item (cast `/Game/Assets/DataAssets/PrimaryDataAssets/PDA_StaticMeshItem` (`self.AdditionalData`)))
  (set `local.StaticMeshData` _aspda_static_mesh_item)
  (bind _returnvalue (`AddComponent|NODE_AddStaticMeshComponent-10` :`RelativeTransform` (`KismetMathLibrary.MakeTransform` (0.0 0.0 0.0) (struct) (`/Game/Assets/DataAssets/PrimaryDataAssets/PDA_AdditionalInfo.Scale` _aspda_static_mesh_item))))
  (`StaticMeshComponent.SetStaticMesh` _returnvalue (`/Game/Assets/DataAssets/PrimaryDataAssets/PDA_StaticMeshItem.StaticMesh` (`local.StaticMeshData`)))
  (`/Engine/EditorBlueprintResources/StandardMacros.IsValid` _overridematerial
    (:`Is Valid`
      (`PrimitiveComponent.SetMaterial` _returnvalue 0 _overridematerial))))

(fn `PickUp`
  (`self.K2_DestroyActor`))

(fn `UserConstructionScript`
  (bind (_itemdata_datatable _itemdata_rowname) (break `DataTableRowHandle` (`self.ItemData`)))
  (bind _returnvalue (`|GetDataTableRow` _itemdata_datatable _itemdata_rowname)
    (:`then`
      (bind _output_get (set `self.Item` _returnvalue))
      (bind _output_get_2 (set `self.AdditionalData` (`.AdditionalData_17_878544914C39EEAAD6E376B2D90F63F1` (break `/Game/Blueprints/Structures/S_Item` _output_get))))
      (if (`KismetMathLibrary.ClassIsChildOf` (`GameplayStatics.GetObjectClass` _output_get_2) "/Game/Assets/DataAssets/PrimaryDataAssets/PDA_StaticMeshItem.PDA_StaticMeshItem_C")
        (`self.AddStaticMesh`)
        (else
          (`self.AddSkeletalMesh`))))))