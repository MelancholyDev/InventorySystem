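; BP_QuestDoor is a usable door that swings open or closed each time it is used.
; BeginPlay stores the starting rotation, and UseActor flips IsOpening to play or reverse the OpenDoor timeline.
; The timeline's update adds its AddRotation track to the starting yaw and rotates the whole actor.
; Despite the name, it contains no quest logic of its own.
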(event `self.ReceiveBeginPlay`
  (set `self.StartRotation` (`self.K2_GetActorRotation`)))

(fn `UseActor`
  (bind _output_get (set `self.IsOpening` (not (`self.IsOpening`))))
  (if _output_get
    (`TimelineComponent.Play` (`self.OpenDoor`))
    (else
      (`TimelineComponent.Reverse` (`self.OpenDoor`)))))

(fn `UserConstructionScript`
  (`parent.UserConstructionScript`))