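; Base usable world actor that only activates when the player's inventory holds a required quest item.
; A Box overlap registers and unregisters the actor with the player's BP_InteractComponent.
; On Use, it looks up the QuestItem data table row and asks BP_InventoryComponent whether one item of that name is held.
; If so, it calls UseActor, which is empty here.
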(event `/Game/Blueprints/Interfaces/BPI_UsableItem.Use`
  (if (`self.CheckContainItem`)
    (`self.UseActor`)))

(event `self.Box.OnComponentBeginOverlap`
  (params (OverlappedComponent :type "PrimitiveComponent Object Reference") (OtherActor :type "Actor Object Reference") (OtherComp :type "PrimitiveComponent Object Reference") (OtherBodyIndex :type Integer) (bFromSweep :type Boolean) (SweepResult :type "HitResult Structure (by ref)"))
  (if (== OtherActor (`GameplayStatics.GetPlayerPawn` 0))
    (`/Game/Blueprints/Components/BP_InteractComponent.AddItem` (`self.GetComponentByClass` (`GameplayStatics.GetPlayerPawn` 0) "/Game/Blueprints/Components/BP_InteractComponent.BP_InteractComponent_C") self)))

(event `self.Box.OnComponentEndOverlap`
  (params (OverlappedComponent :type "PrimitiveComponent Object Reference") (OtherActor :type "Actor Object Reference") (OtherComp :type "PrimitiveComponent Object Reference") (OtherBodyIndex :type Integer))
  (if (== OtherActor (`GameplayStatics.GetPlayerPawn` 0))
    (`/Game/Blueprints/Components/BP_InteractComponent.DeleteItem` (`self.GetComponentByClass` (`GameplayStatics.GetPlayerPawn` 0) "/Game/Blueprints/Components/BP_InteractComponent.BP_InteractComponent_C") self)))

(fn `CheckContainItem`
  (returns (IsContain :type Boolean))
  (bind (_questitem_datatable _questitem_rowname) (break `DataTableRowHandle` (`self.QuestItem`)))
  (bind _returnvalue (`|GetDataTableRow` _questitem_datatable _questitem_rowname)
    (:`then`
      (bind _structout (setmembers `/Game/Blueprints/Structures/S_Item` :`StructRef` _returnvalue))
      (bind _iscontain (`/Game/Blueprints/Components/BP_InventoryComponent.ContainObjectNum` (`self.GetComponentByClass` (`GameplayStatics.GetPlayerPawn` 0) "/Game/Blueprints/Components/BP_InventoryComponent.BP_InventoryComponent_C") (break `/Game/Blueprints/Structures/S_Item` _structout) 1))
      (return _iscontain))))

(fn `UseActor`)

(fn `UserConstructionScript`
  (`parent.UserConstructionScript`))