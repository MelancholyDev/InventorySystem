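; BP_Weapon is a usable item that fires when used, provided the player carries enough ammo.
; On Use it looks up the ammo item through a data table row handle and checks the player pawn's BP_InventoryComponent for the per-shot amount.
; A successful shot plays a sound at the weapon's location and removes that ammo from the inventory.
; The file contains no projectile, trace or damage logic.
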(event `/Game/Blueprints/Interfaces/BPI_UsableItem.Use`
  (if (`self.IsEnoughAmmo`)
    (`self.Shot`)))

(fn `IsEnoughAmmo`
  (returns (IsEnough :type Boolean))
  (bind (_ammo_datatable _ammo_rowname) (break `DataTableRowHandle` (`self.Ammo`)))
  (bind _returnvalue (`|GetDataTableRow` _ammo_datatable _ammo_rowname)
    (:`then`
      (bind _structout (setmembers `/Game/Blueprints/Structures/S_Item` :`StructRef` _returnvalue))
      (bind _iscontain (`/Game/Blueprints/Components/BP_InventoryComponent.ContainObjectNum` (`self.GetComponentByClass` (`GameplayStatics.GetPlayerPawn` 0) "/Game/Blueprints/Components/BP_InventoryComponent.BP_InventoryComponent_C") (break `/Game/Blueprints/Structures/S_Item` _structout) (`self.AmmoToShotOnce`)))
      (return _iscontain))))

(fn `Shot`
  (bind (_ammo_datatable _ammo_rowname) (break `DataTableRowHandle` (`self.Ammo`)))
  (`GameplayStatics.PlaySoundAtLocation` (`self.ShotSound`) (`self.K2_GetActorLocation`) (struct) 1.0 1.0 0.0 null null null null)
  (bind _returnvalue (`|GetDataTableRow` _ammo_datatable _ammo_rowname)
    (:`then`
      (bind _structout (setmembers `/Game/Blueprints/Structures/S_Item` :`StructRef` _returnvalue))
      (`/Game/Blueprints/Components/BP_InventoryComponent.DeleteObjectNum` (`self.GetComponentByClass` (`GameplayStatics.GetPlayerPawn` 0) "/Game/Blueprints/Components/BP_InventoryComponent.BP_InventoryComponent_C") (break `/Game/Blueprints/Structures/S_Item` _structout) (`self.AmmoToShotOnce`)))))

(fn `UserConstructionScript`
  (`parent.UserConstructionScript`))